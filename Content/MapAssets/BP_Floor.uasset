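; Floor area that lights up while the player is inside it and hides the other actors on it otherwise.
; Box overlaps with "Player"-tagged actors set IsVisible and call SetLight, which swaps the Paper2D sprite between lit and shadow and updates tracked actors' visibility.
; Other actors join ActorsInFloor on entry, matching the floor's visibility, and are removed and hidden on exit.
; The construction script applies the same logic from IsVisible.
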(event OnComponentBeginOverlap(Box)
  (params (OtherActor :type Actor%20Object%20Reference) (OtherComp :type Primitive%20Component%20Object%20Reference) (OtherBodyIndex :type Integer) (bFromSweep :type Boolean) (SweepResult :type Hit%20Result%20Structure%20%28by%20ref%29))
  (if (Actor|ActorHasTag OtherActor "Player")
    (bind _output_get (Variables|Default|SetisVisible true))
    (CallFunction|SetLight _output_get)
    (else
      (Utilities|Array|Add (Variables|Default|GetActorsInFloor) OtherActor)
      (Rendering|SetActorHiddenInGame OtherActor (not (Variables|Default|GetisVisible))))))

(event OnComponentEndOverlap(Box)
  (params (OtherActor :type Actor%20Object%20Reference) (OtherComp :type Primitive%20Component%20Object%20Reference) (OtherBodyIndex :type Integer))
  (if (Actor|ActorHasTag OtherActor "Player")
    (bind _output_get (Variables|Default|SetisVisible false))
    (CallFunction|SetLight _output_get)
    (else
      (Utilities|Array|RemoveItem (Variables|Default|GetActorsInFloor) OtherActor)
      (Rendering|SetActorHiddenInGame OtherActor true))))

(event EventActorBeginOverlap
  (params (OtherActor :type Actor%20Object%20Reference)))

(event EventTick
  (params (DeltaSeconds :type Float%20%28single-precision%29)))

(fn ConstructionScript
  (bind _papersprite (Variables|Default|GetPaperSprite))
  (if (Variables|Default|GetisVisible)
    (Rendering|Components|Sprite|SetSprite _papersprite (Variables|Default|GetInLightSprite))
    (else
      (Rendering|Components|Sprite|SetSprite _papersprite (Variables|Default|GetInShadowSprite))))
  (for _array_element (Variables|Default|GetActorsInFloor)
    (Rendering|SetActorHiddenInGame _array_element (not (Variables|Default|GetisVisible)))))

(fn SetLight
  (params (IsLit :type Boolean))
  (bind _papersprite (Variables|Default|GetPaperSprite))
  (if IsLit
    (Rendering|Components|Sprite|SetSprite _papersprite (Variables|Default|GetInLightSprite))
    (else
      (Rendering|Components|Sprite|SetSprite _papersprite (Variables|Default|GetInShadowSprite))))
  (for _array_element (Variables|Default|GetActorsInFloor)
    (Rendering|SetActorHiddenInGame _array_element (not IsLit))))