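; Blueprint function library of utilities for AgentSlick, providing a MoveAgentToLocation helper that moves the player's agent.
; It casts player controller 0 to AgentSlickPlayerController and stops its current movement.
; It then either teleports the controlled pawn or sends it via SimpleMoveToLocation, using only the target's X and Y and keeping the pawn's current Z.
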(fn MoveAgenttoLocation
  (params (Object :type Actor%20Object%20Reference) (Location :type Vector) (Teleport :type Boolean))
  (bind (_x _y) (Math|Vector|BreakVector Location))
  (bind _asagent_slick_player_controller (Utilities|Casting|CastToAgentSlickPlayerController (Game|GetPlayerController Object)))
  (AI|Navigation|StopMovement _asagent_slick_player_controller)
  (if Teleport
    (Transformation|SetActorLocation (Pawn|GetControlledPawn _asagent_slick_player_controller) (Math|Vector|MakeVector _x _y (.Z (Math|Vector|BreakVector (Transformation|GetActorLocation (Pawn|GetControlledPawn _asagent_slick_player_controller))))) false true)
    (else
      (AI|Navigation|SimpleMovetoLocation _asagent_slick_player_controller (Math|Vector|MakeVector _x _y (.Z (Math|Vector|BreakVector (Transformation|GetActorLocation (Pawn|GetControlledPawn _asagent_slick_player_controller)))))))))